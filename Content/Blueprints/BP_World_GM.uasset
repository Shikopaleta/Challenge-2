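; World game mode that handles checkpoints, player respawn and resetting the level to its initial state.
; On BeginPlay it sets game-only input and records the current mode on the game instance.
; Checkpoints only advance to higher IDs, and respawn teleports BP_WorldCharacter to the current one's SpawnPoint, or the first PlayerStart found if none is set.
; Reset broadcasts a message to every actor implementing I_WorldMessages.
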(event Custom|Checkpoint%20Reached
  (params (Checkpoint%20Actor :type BP%20Checkpoint%20Object%20Reference))
  (Utilities|IsValid (Variables|Default|GetCurrent%20Checkpoint)
    (:Is%20Valid
      (if (> (Variables|/Game/Blueprints/Save/BP_Checkpoint.BP_Checkpoint_C|GetID Checkpoint%20Actor) (Variables|/Game/Blueprints/Save/BP_Checkpoint.BP_Checkpoint_C|GetID (Variables|Default|GetCurrent%20Checkpoint)))
        (bind _output_get (Variables|Default|SetCurrent%20Checkpoint Checkpoint%20Actor))
        (Development|PrintString (Utilities|String|Append "Checkpoint with ID " (Utilities|String|ToString(Integer) (Variables|/Game/Blueprints/Save/BP_Checkpoint.BP_Checkpoint_C|GetID _output_get)) " reached") :!label _label)))
    (:Is%20Not%20Valid
      (Variables|Default|SetCurrent%20Checkpoint Checkpoint%20Actor)
      (goto _label))))

(event Custom|Reset%20Game%20to%20initial%20state
  (bind _outactors (Actor|GetAllActorswithInterface "/Game/Blueprints/Interfaces/I_WorldMessages.I_WorldMessages_C"))
  (for _array_element _outactors
    (Class|IWorldMessages|ResettoInitialState(Message) _array_element)))

(event Custom|Respawn%20Player
  (bind _current_checkpoint (Variables|Default|GetCurrent%20Checkpoint))
  (bind _spawn_point (Variables|/Game/Blueprints/Save/BP_Checkpoint.BP_Checkpoint_C|GetSpawn%20Point _current_checkpoint))
  (Utilities|IsValid (Variables|Default|GetCurrent%20Checkpoint)
    (:Is%20Valid
      (bind _asbp_world_character (Utilities|Casting|CastToBP_WorldCharacter (Game|GetPlayerCharacter 0)))
      (Default|Respawn _asbp_world_character)
      (Transformation|SetActorLocationAndRotation _asbp_world_character (Transformation|GetWorldLocation _spawn_point) (Transformation|GetWorldRotation _spawn_point)))
    (:Is%20Not%20Valid
      (bind _outactors (Actor|GetAllActorsOfClass "/Script/Engine.PlayerStart"))
      (bind _asbp_world_character_2 (Utilities|Casting|CastToBP_WorldCharacter (Game|GetPlayerCharacter 0)))
      (Default|Respawn _asbp_world_character_2)
      (Transformation|SetActorLocationAndRotation _asbp_world_character_2 (Transformation|GetActorLocation (Utilities|Array|Get(acopy) _outactors)) (Transformation|GetActorRotation (Utilities|Array|Get(acopy) _outactors))))))

(event EventBeginPlay
  (Input|SetInputModeGameOnly (Game|GetPlayerController 0))
  (Variables|/Game/Blueprints/BP_GameInstance.BP_GameInstance_C|SetGame%20Mode (CallFunction|GetNewGameInstance) "NewEnumerator1"))

(fn ConstructionScript)