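; BP_ControlBox is an interactive control box that activates a linked Platform once all its linked valves are engaged.
; Valveengaged checks every valve in the Valves array and disables them all when each is engaged.
; Player interaction then turns off the box's interaction collision and activates the Platform.
; It can also reset the valves or its own state, and prints a warning on BeginPlay if no valid Platform is assigned.
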(event Custom|Valve%20engaged
  (bind _array_element (Utilities|Array|ForEachLoopwithBreak (Variables|Default|GetValves) :!label _label)
    (:LoopBody
      (bind _output_get (Variables|Default|SetAll%20Valves%20engaged (Variables|/Game/Blueprints/Interactivebjects/BP_Valve.BP_Valve_C|GetValve%20Engaged? _array_element)))
      (if (not _output_get)
        (goto _label Break)))
    (:Completed
      (if (Variables|Default|GetAll%20Valves%20engaged)
        (for _array_element_2 (Variables|Default|GetValves)
          (Default|DisableValve _array_element_2))))))

(event Custom|Reset%20Valves
  (Development|PrintString "All Valves reset")
  (for _array_element (Variables|Default|GetValves)
    (Default|ResetValve _array_element)))

(event EventBeginPlay
  (Utilities|IsValid (Variables|Default|GetPlatform)
    (:Is%20Not%20Valid
      (Development|PrintString (Utilities|String|Append "Platform in object " (Utilities|GetDisplayName self) " is invalid, select one.")))))

(event EventOnPlayerInteract
  (if (Variables|Default|GetAll%20Valves%20engaged)
    (Collision|SetCollisionEnabled (Variables|Default|GetInteractive%20Collision) "NoCollision")
    (Development|PrintString "Control  box engaged")
    (Default|Activate (Variables|Default|GetPlatform))))

(event EventResettoInitialState
  (Variables|Default|SetAll%20Valves%20engaged false)
  (Collision|SetCollisionEnabled (Variables|Default|GetInteractive%20Collision) "QueryOnly"))

(fn ConstructionScript)