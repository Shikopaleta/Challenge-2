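; Base collectible item that the player picks up by interacting with it, adding its item type to the world player controller's inventory.
; Pickup happens only while the item is not taken, then flags it taken and clears its static mesh rather than destroying the actor.
; Resetting to the initial state restores the configured mesh and removes the item from the inventory.
; The construction script applies that mesh through a DoOnce.
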(event EventResettoInitialState
  (Variables|Default|Setis%20Taken? false)
  (Components|StaticMesh|SetStaticMesh (Variables|Default|GetSM_lever_low) (Variables|Default|GetItem%20Static%20Mesh))
  (bind _asbp_world_player_controller (Utilities|Casting|CastToBP_WorldPlayerController (Game|GetPlayerController 0)))
  (Default|RemoveItemfromInventory _asbp_world_player_controller (Variables|Default|GetItem%20type)))

(event EventOnPlayerInteract
  (if (not (Variables|Default|Getis%20Taken?))
    (bind _asbp_world_player_controller (Utilities|Casting|CastToBP_WorldPlayerController (Game|GetPlayerController 0)))
    (Default|AddItemtoInventory _asbp_world_player_controller (Variables|Default|GetItem%20type))
    (Variables|Default|Setis%20Taken? true)
    (Components|StaticMesh|SetStaticMesh (Variables|Default|GetSM_lever_low) 0)))

(fn ConstructionScript
  (Utilities|FlowControl|DoOnce false
    (:Completed
      (Components|StaticMesh|SetStaticMesh (Variables|Default|GetSM_lever_low) (Variables|Default|GetItem%20Static%20Mesh)))))