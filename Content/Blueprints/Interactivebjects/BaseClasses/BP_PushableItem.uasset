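; Base pushable item that the player grabs and moves around, with a reset to its construction-time transform.
; On interact, a line trace finds the touched face and a timeline slides and turns the player to face it at AttachDistance, then registers the item as GrabbedActor.
; MoveActor sweeps the item to stay in front of the player, detaching when that move fails and the player is beyond AttachDistance.
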(event Custom|Detach%20From%20Character
  (bind _asbp_world_character (Utilities|Casting|CastToBP_WorldCharacter (Game|GetPlayerCharacter 0)))
  (Variables|/Game/Blueprints/Player/BP_WorldCharacter.BP_WorldCharacter_C|SetGrabbedActor _asbp_world_character 0)
  (Variables|/Script/Engine.CharacterMovementComponent|SetbOrientRotationToMovement (Variables|/Script/Engine.Character|GetCharacterMovement _asbp_world_character) true))

(event EventOnPlayerInteract
  (bind _returnvalue (Game|GetPlayerCharacter 0))
  (bind _returnvalue_2 (Game|GetPlayerCharacter 0))
  (Variables|/Script/Engine.CharacterMovementComponent|SetbOrientRotationToMovement (Variables|/Script/Engine.Character|GetCharacterMovement _returnvalue) false)
  (Input|DisableInput _returnvalue 0)
  (bind _outhit (Collision|LineTraceByChannel (Transformation|GetActorLocation _returnvalue) (Transformation|GetActorLocation) "TraceTypeQuery1" false (Utilities|Array|MakeArray (Game|GetPlayerCharacter 0)) "None" false "(R=1.000000,G=0.000000,B=0.000000,A=1.000000)" "(R=0.000000,G=1.000000,B=0.000000,A=1.000000)" 2.0))
  (bind _alpha (Timeline|Move%20to PlayFromStart)
    (:Update
      (|MovetoPlace _alpha (.impactnormal _outhit)))
    (:Finished
      (Input|EnableInput _returnvalue_2 (Game|GetPlayerController 0))
      (bind _asbp_world_character (Utilities|Casting|CastToBP_WorldCharacter _returnvalue_2))
      (Variables|/Game/Blueprints/Player/BP_WorldCharacter.BP_WorldCharacter_C|SetGrabbedActor _asbp_world_character self))))

(event EventResettoInitialState
  (Transformation|SetActorTransform (Variables|Default|GetInitial%20Transform)))

(fn ConstructionScript
  (Variables|Default|SetInitial%20Transform (Transformation|GetActorTransform))
  (if (Variables|Default|GetDraw%20Debug%20Attach%20Distance)
    (Rendering|Debug|DrawDebugLine (Transformation|GetActorLocation) (+ (Transformation|GetActorLocation) (* (Transformation|GetActorForwardVector) (Variables|Default|GetAttach%20Distance))) "(R=1.000000,G=0.000000,B=0.000000,A=1.000000)" 2.0 5.0)
    (Variables|Default|SetDraw%20Debug%20Attach%20Distance false)))

(fn MoveActor
  (bind _returnvalue (Game|GetPlayerCharacter 0))
  (bind _returnvalue_2 (Game|GetPlayerCharacter 0))
  (bind _attach_distance (Variables|Default|GetAttach%20Distance))
  (bind _returnvalue_3 (Transformation|GetDistanceTo _returnvalue))
  (bind _returnvalue_4 (Transformation|GetActorForwardVector _returnvalue_2))
  (bind _returnvalue_5 (Transformation|GetActorLocation _returnvalue_2))
  (bind _returnvalue_6 (* _returnvalue_4 _attach_distance))
  (bind _returnvalue_7 (+ _returnvalue_6 _returnvalue_5))
  (bind _returnvalue_8 (Transformation|SetActorLocation (Math|Vector|MakeVector (.x _returnvalue_7) (.y _returnvalue_7) (.z (Transformation|GetActorLocation))) true false))
  (Rendering|Debug|DrawDebugString _returnvalue_5 (Utilities|String|ToString(Float) _returnvalue_3) 0 "(R=1.000000,G=1.000000,B=1.000000,A=1.000000)")
  (if _returnvalue_8
    _
    (elif (> _returnvalue_3 (Variables|Default|GetAttach%20Distance))
      (CallFunction|DetachfromCharacter)))
  (return))