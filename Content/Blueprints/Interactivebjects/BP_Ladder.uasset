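; Interactable ladder that the player character climbs between two arrow-marked ends.
; Interacting turns off the character's collision and gravity and the upper-floor collision, then a timeline aligns the player to the nearer arrow.
; Climb input moves the player vertically, only toward the far end until a threshold distance is passed.
; After that, movement is free both ways and a destination check triggers detach, which restores collision and gravity.
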(event Custom|Start%20Climbing
  (params (Value :type Float%20%28single-precision%29))
  (bind _returnvalue (Game|GetPlayerCharacter 0))
  (bind _returnvalue_2 (Utilities|Time|GetWorldDeltaSeconds))
  (bind _climb_speed (Variables|Default|GetClimb%20Speed))
  (bind _returnvalue_3 (* Value _climb_speed))
  (bind _returnvalue_4 (* _returnvalue_3 _returnvalue_2))
  (if (Variables|Default|Getthreshold%20passed?)
    (Transformation|AddActorWorldOffset _returnvalue (Math|Vector|MakeVector 0.0 0.0 _returnvalue_4))
    (if (|Checkifitisindistancetodestination)
      (CallFunction|Detach))
    (elif (< (Math|Vector|VectorLength (- (+ (Transformation|GetActorLocation (Game|GetPlayerCharacter 0)) (Math|Vector|MakeVector 0.0 0.0 _returnvalue_4)) (Variables|Default|GetOther%20point))) (Math|Vector|VectorLength (- (Transformation|GetActorLocation (Game|GetPlayerCharacter 0)) (Variables|Default|GetOther%20point))))
      (Transformation|AddActorWorldOffset _returnvalue (Math|Vector|MakeVector 0.0 0.0 _returnvalue_4))
      (if (> (Math|Vector|VectorLength (- (Transformation|GetActorLocation (Game|GetPlayerCharacter 0)) (Variables|Default|GetAttached%20Loc))) 75.0)
        (Variables|Default|Setthreshold%20passed? true)
        (Development|PrintString "threshold passed")))))

(event Custom|Stop%20Climbing)

(event Custom|Detach
  (bind _asbp_world_character (Utilities|Casting|CastToBP_WorldCharacter (Game|GetPlayerCharacter 0)))
  (Variables|/Game/Blueprints/Player/BP_WorldCharacter.BP_WorldCharacter_C|SetLadder _asbp_world_character 0)
  (Variables|/Script/Engine.CharacterMovementComponent|SetGravityScale (Variables|/Script/Engine.Character|GetCharacterMovement _asbp_world_character) 1.0)
  (Collision|SetActorEnableCollision _asbp_world_character true)
  (Variables|Default|Setthreshold%20passed? false)
  (Collision|SetCollisionEnabled (Variables|Default|GetUpper%20Floor%20Collision) "QueryAndPhysics"))

(event EventOnPlayerInteract
  (bind _asbp_world_character (Utilities|Casting|CastToBP_WorldCharacter (Game|GetPlayerCharacter 0)))
  (Input|DisableInput _asbp_world_character 0)
  (Variables|/Game/Blueprints/Player/BP_WorldCharacter.BP_WorldCharacter_C|SetLadder _asbp_world_character self)
  (Collision|SetActorEnableCollision _asbp_world_character false)
  (Variables|/Script/Engine.CharacterMovementComponent|SetGravityScale (Variables|/Script/Engine.Character|GetCharacterMovement _asbp_world_character) 0.0)
  (Variables|/Script/Engine.MovementComponent|SetVelocity (Variables|/Script/Engine.Character|GetCharacterMovement _asbp_world_character) "0, 0, 0")
  (Variables|Default|Setthreshold%20passed? false)
  (|MovePlayertoPosition)
  (Collision|SetCollisionEnabled (Variables|Default|GetUpper%20Floor%20Collision) "NoCollision")
  (Input|EnableInput (Game|GetPlayerCharacter 0) (Game|GetPlayerController 0)))

(fn ConstructionScript)