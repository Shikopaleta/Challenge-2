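; BP_Platform is an interactive moving platform that slides to a landing point when activated.
; Activate plays a timeline that lerps the static mesh's relative location from its origin to the LandingPoint component's position, without sweeping.
; The construction script sets the timeline play rate to the inverse of a Time variable, so Time sets travel duration.
; Reset events snap the mesh back to its origin.
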(event Custom|Activate
  (bind _alpha (Timeline|Move%20Platform PlayFromStart)
    (:Update
      (Transformation|SetRelativeLocation (Variables|Default|GetStaticMesh) (Math|Vector|Lerp(Vector) "0, 0, 0" (Variables|/Script/Engine.SceneComponent|GetRelativeLocation (Variables|Default|GetLanding%20point)) _alpha) false false))))

(event EventResettoInitialState
  (Transformation|SetRelativeLocation (Variables|Default|GetStaticMesh) "0, 0, 0" false false))

(event EventOnReset
  (Transformation|SetRelativeLocation (Variables|Default|GetStaticMesh) "0, 0, 0" false false))

(fn ConstructionScript
  (Components|Timeline|SetPlayRate (Variables|Default|GetMove%20Platform) (/ 1.0 (Variables|Default|GetTime))))