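; BP_Valve is an interactable valve that depends on a referenced PowerBox for power.
; On BeginPlay it prints a warning naming the actor if the PowerBox reference is invalid.
; When the player interacts, it checks the box's Powered flag and prints either an engaged or a needs-power message.
; Interaction currently only prints debug strings, with no valve movement or other effect.
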(event EventBeginPlay
  (Utilities|IsValid (Variables|Default|GetPower%20Box)
    (:Is%20Not%20Valid
      (Development|PrintString (Utilities|String|Append "Power Box is invalid in actor: " (Utilities|GetDisplayName self))))))

(event EventOnPlayerInteract
  (if (Variables|/Game/Blueprints/Interactivebjects/BP_PowerGenerator.BP_PowerGenerator_C|GetPowered? (Variables|Default|GetPower%20Box))
    (Development|PrintString "valves engaged")
    (else
      (Development|PrintString "Valves need power"))))

(fn ConstructionScript)