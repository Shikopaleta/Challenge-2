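; Interactive power box that the player turns on after fitting it with a lever from their inventory.
; Interacting without a fitted lever checks the world player controller's inventory, consumes the item and sets the lever mesh.
; A later interaction sets Powered, plays a sound and, after a short delay, a radial camera shake, with debug prints as feedback.
; A reset event clears both state flags and the lever mesh.
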(event EventResettoInitialState
  (Variables|Default|SetHas%20Lever? false)
  (Variables|Default|SetPowered? false)
  (Components|StaticMesh|SetStaticMesh (Variables|Default|GetSM_lever_low) 0))

(event EventOnPlayerInteract
  (bind _returnvalue (Game|GetPlayerController 0))
  (bind _returnvalue_2 (Transformation|GetActorLocation))
  (bind _asbp_world_player_controller (Utilities|Casting|CastToBP_WorldPlayerController _returnvalue))
  (if (Variables|Default|GetHas%20Lever?)
    (if (not (Variables|Default|GetPowered?))
      (Variables|Default|SetPowered? true)
      (Audio|PlaySoundatLocation 0 _returnvalue_2)
      (Utilities|FlowControl|Delay 0.2)
      (Camera|PlayWorldCameraShake 0 _returnvalue_2 0.0 7e+02)
      (Development|PrintString "Power generator turned on")
      (else
        (Development|PrintString "Power generator already on")))
    (elif (Default|IsIteminInventory _asbp_world_player_controller "NewEnumerator0")
      (Variables|Default|SetHas%20Lever? true)
      (Default|RemoveItemfromInventory _asbp_world_player_controller "NewEnumerator0")
      (Components|StaticMesh|SetStaticMesh (Variables|Default|GetSM_lever_low) "/Game/Assets/Assets/05_lever/lever_low.lever_low")
      (Development|PrintString "Lever penetrated")
      (else
        (Development|PrintString "Lever missing; if anything, give hint in this node.")))))

(fn ConstructionScript)