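; BP_BaseAiPawn is a base AI pawn that tracks whether it is idle and whether the player is nearby.
; Idle and StopIdle events set and clear the IsIdle flag.
; ProximityCollision overlaps are filtered to player character 0 and routed through OnPlayerInProximity and OnPlayerNotInProximity events, which update PlayerIsInProximity.
; It only maintains these flags and does not act on them.
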(event OnComponentBeginOverlap(ProximityCollision)
  (params (OverlappedComponent :type Primitive%20Component%20Object%20Reference) (OtherActor :type Actor%20Object%20Reference) (OtherComp :type Primitive%20Component%20Object%20Reference) (OtherBodyIndex :type Integer) (bFromSweep :type Boolean) (SweepResult :type Hit%20Result%20Structure%20%28by%20ref%29))
  (if (== OtherActor (Game|GetPlayerCharacter 0))
    (CallFunction|OnPlayerinProximity)))

(event OnComponentEndOverlap(ProximityCollision)
  (params (OverlappedComponent :type Primitive%20Component%20Object%20Reference) (OtherActor :type Actor%20Object%20Reference) (OtherComp :type Primitive%20Component%20Object%20Reference) (OtherBodyIndex :type Integer))
  (if (== (Game|GetPlayerCharacter 0) OtherActor)
    (CallFunction|OnPlayerNotinProximity)))

(event Custom|Idle
  (Variables|Default|SetIs%20Idle true))

(event Custom|On%20Player%20In%20Proximity
  (Variables|Default|SetPlayer%20Is%20In%20Proximity true))

(event Custom|On%20Player%20Not%20In%20Proximity
  (Variables|Default|SetPlayer%20Is%20In%20Proximity false))

(event Custom|Stop%20Idle
  (Variables|Default|SetIs%20Idle false))

(fn ConstructionScript)