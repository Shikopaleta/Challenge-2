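; Security camera pawn that sweeps for the player and kills them if they stay in sight.
; Idle ping-pongs the pivot's yaw, line-tracing every 0.2s and reporting visible players inside VisionCollision to BP_CameraController.
; LookAtPlayer turns the spotlight red and starts timeline-driven tracking, with three-second delays before killing or reporting lost sight.
; Proximity events update the controller; leaving also stops idle and tracking, saving the rotation for a smooth return.
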(event Custom|Look%20At%20Player
  (CallFunction|StopIdle)
  (Rendering|Components|Light|SetLightColor (Variables|Default|GetSpotLight) "(R=1.000000,G=0.143001,B=0.103198,A=1.000000)" true)
  (Variables|Default|SetIdle%20Rot (Variables|/Script/Engine.SceneComponent|GetRelativeRotation (Variables|Default|GetCameraPivot)))
  (|FollowPlayer))

(event Custom|Start%20Loop
  (bind _returnvalue (Game|GetPlayerCharacter 0))
  (if (Variables|Default|GetIs%20Idle)
    (bind _outhit (Collision|LineTraceByChannel (Transformation|GetActorLocation) (Transformation|GetActorLocation (Game|GetPlayerCharacter 0)) "TraceTypeQuery1" false 0 "None"))
    (Utilities|FlowControl|Sequence
      (:then_0
        (if (== (.hitactor _outhit) _returnvalue)
          (if (Collision|IsOverlappingActor (Variables|Default|GetVision%20Collision) _returnvalue :!class /Script/Engine.PrimitiveComponent)
            (bind _asbp_camera_controller (Utilities|Casting|CastToBP_CameraController (Pawn|GetController)))
            (Default|SetIsPlayeronSight _asbp_camera_controller true))))
      (:then_1
        (Utilities|FlowControl|Delay 0.2)
        (CallFunction|StartLoop)))))

(event Custom|Stop%20Looking%20At%20Player
  (Variables|Default|SetLast%20Rot (Variables|/Script/Engine.SceneComponent|GetRelativeRotation (Variables|Default|GetCameraPivot)))
  (Rendering|Components|Light|SetLightColor (Variables|Default|GetSpotLight) "(R=1.000000,G=0.844394,B=0.562500,A=1.000000)" true)
  (|FollowPlayer) ; enters at Stop
)

(event EventBeginPlay)

(event EventStopIdle
  (bind _camera_y_rotation (Variables|Default|GetCamera%20Y%20Rotation))
  (|CallParentFunction)
  (Audio|Components|Audio|Stop (Variables|Default|GetIdle%20Sound%20Component))
  (bind (_direction _alpha) (Timeline|Idle%20Loop Stop)
    (:Update
      (Transformation|SetRelativeRotation (Variables|Default|GetCameraPivot) (Math|Rotator|Lerp(Rotator) (Math|Rotator|MakeRotator 0.0 _camera_y_rotation 6e+01) (Math|Rotator|MakeRotator 0.0 _camera_y_rotation -6e+01) _alpha true) false false))
    (:Finished
      (switch Utilities|FlowControl|Switch|SwitchonETimelineDirection _direction
        (:Forward
          (Timeline|Idle%20Loop ReverseFromEnd))
        (:Backward
          (Timeline|Idle%20Loop PlayFromStart))))))

(event EventOnPlayerinProximity
  (|CallParentFunction)
  (bind _asbp_camera_controller (Utilities|Casting|CastToBP_CameraController (Pawn|GetController)))
  (Default|SetIsPlayerinProximity _asbp_camera_controller true))

(event EventOnPlayerNotinProximity
  (|CallParentFunction)
  (CallFunction|StopIdle)
  (CallFunction|StopLookingatPlayer)
  (bind _asbp_camera_controller (Utilities|Casting|CastToBP_CameraController (Pawn|GetController)))
  (Default|SetIsPlayerinProximity _asbp_camera_controller false)
  (Variables|Default|SetIs%20Player%20Seen? false))

(event EventIdle
  (bind _camera_y_rotation (Variables|Default|GetCamera%20Y%20Rotation))
  (|CallParentFunction)
  (CallFunction|StopLookingatPlayer)
  (bind _alpha (Timeline|Return%20to%20rot PlayFromStart)
    (:Update
      (Transformation|SetRelativeRotation (Variables|Default|GetCameraPivot) (Math|Rotator|Lerp(Rotator) (Variables|Default|GetLast%20Rot) (Variables|Default|GetIdle%20Rot) _alpha true) false false))
    (:Finished
      (Audio|Components|Audio|Play (Variables|Default|GetIdle%20Sound%20Component) 0.0)
      (CallFunction|StartLoop)
      (switch Utilities|FlowControl|Switch|SwitchonETimelineDirection (stale _direction)
        (:Forward
          (bind (_direction _alpha_2) (Timeline|Idle%20Loop Play)
            (:Update
              (Transformation|SetRelativeRotation (Variables|Default|GetCameraPivot) (Math|Rotator|Lerp(Rotator) (Math|Rotator|MakeRotator 0.0 _camera_y_rotation 6e+01) (Math|Rotator|MakeRotator 0.0 _camera_y_rotation -6e+01) _alpha_2 true) false false))
            (:Finished
              (switch Utilities|FlowControl|Switch|SwitchonETimelineDirection _direction
                (:Forward
                  (Timeline|Idle%20Loop ReverseFromEnd))
                (:Backward
                  (Timeline|Idle%20Loop PlayFromStart))))))
        (:Backward
          (Timeline|Idle%20Loop Reverse))))))

(fn ConstructionScript
  (Transformation|SetRelativeRotation (Variables|Default|GetCameraPivot) (Math|Rotator|MakeRotator 0.0 (Variables|Default|GetCamera%20Y%20Rotation) 0.0) false false))