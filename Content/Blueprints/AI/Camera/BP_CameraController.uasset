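; AI controller for a camera, which runs the BT_Camera behavior tree on BeginPlay.
; Two events act as setters that write player sight and proximity flags to Blackboard booleans, after checking that the Blackboard is valid.
; The controller holds no detection logic of its own and only passes on the values it receives.
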(event Custom|Set%20Is%20Player%20On%20Sight
  (params (BoolValue :type Boolean))
  (bind _self self)
  (bind _returnvalue (AI|GetBlackboard _self))
  (Utilities|IsValid _returnvalue
    (:Is%20Valid
      (AI|Components|Blackboard|SetValueasBool _returnvalue (Utilities|Name|MakeLiteralName "Is Player Detected?") BoolValue))))

(event Custom|Set%20Is%20Player%20in%20Proximity
  (params (Bool%20Value :type Boolean))
  (bind _self self)
  (bind _returnvalue (AI|GetBlackboard _self))
  (Utilities|IsValid _returnvalue
    (:Is%20Valid
      (AI|Components|Blackboard|SetValueasBool _returnvalue (Utilities|Name|MakeLiteralName "Is Player in Proximity") Bool%20Value))))

(event EventBeginPlay
  (AI|RunBehaviorTree "/Game/Blueprints/AI/Camera/BT_Camera.BT_Camera"))

(fn ConstructionScript)