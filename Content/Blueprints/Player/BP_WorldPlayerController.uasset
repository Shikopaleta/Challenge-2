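; Player controller for the world that handles the pause menu, screen fade and the player's inventory.
; On BeginPlay it takes the menu and fade widgets from the game instance and shows the fade; the pause input toggles the menu, cursor and input mode.
; Inventory functions check, add without duplicates and remove items.
; Hardcoded O and P keys kill the player character and reset the game through the game mode.
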(event EventBeginPlay
  (bind _game_instance (CallFunction|GetNewGameInstance))
  (Variables|Default|SetBPW%20Menu (Variables|/Game/Blueprints/BP_GameInstance.BP_GameInstance_C|GetBPW%20Menu _game_instance))
  (bind _output_get (Variables|Default|SetBPW%20Screen%20Fade (Variables|/Game/Blueprints/BP_GameInstance.BP_GameInstance_C|GetBPW%20Screen%20Fade _game_instance)))
  (UserInterface|Viewport|AddtoViewport _output_get 0))

(event Input|ActionEvents|InputActionPauseMenu
  (params (Key :type Key%20Structure))
  (bind _self self)
  (bind _bpw_menu (Variables|Default|GetBPW%20Menu))
  (:Pressed
    (if (UserInterface|Viewport|IsinViewport (Variables|Default|GetBPW%20Menu))
      (Widget|RemovefromParent _bpw_menu)
      (Input|SetInputModeGameOnly _self)
      (Variables|Default|SetbShowMouseCursor false)
      (else
        (UserInterface|Viewport|AddtoViewport _bpw_menu 0)
        (Input|SetInputModeGameandUI _self (Variables|Default|GetBPW%20Menu) "LockOnCapture" false)
        (Variables|Default|SetbShowMouseCursor true)))))

(event Input|KeyboardEvents|O
  (params (Key :type Key%20Structure))
  (:Pressed
    (bind _asbp_world_character (Utilities|Casting|CastToBP_WorldCharacter (Game|GetPlayerCharacter 0)))
    (Default|KillPlayer _asbp_world_character)))

(event Input|KeyboardEvents|P
  (params (Key :type Key%20Structure))
  (:Pressed
    (bind _asbp_world_gm (Utilities|Casting|CastToBP_World_GM (Game|GetGameMode)))
    (Default|ResetGametoInitialState _asbp_world_gm)))

(fn ConstructionScript)

(fn IsIteminInventory
  (params (Item :type E_InteractiveItems%20Enum :default "NewEnumerator0"))
  (return (select (>= (Utilities|Array|FindItem (Variables|Default|GetInventory) Item) 0) true false)))

(fn AddItemtoInventory
  (params (Item :type E_InteractiveItems%20Enum :default "NewEnumerator0"))
  (if (not (CallFunction|IsIteminInventory Item))
    (Utilities|Array|Add (Variables|Default|GetInventory) Item)))

(fn RemoveItemfromInventory
  (params (Item :type E_InteractiveItems%20Enum :default "NewEnumerator0"))
  (if (CallFunction|IsIteminInventory Item)
    (bind _returnvalue (Utilities|Array|RemoveItem (Variables|Default|GetInventory) Item))
    (return _returnvalue)
    (else
      (return false))))